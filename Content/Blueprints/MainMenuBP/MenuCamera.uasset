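; MenuCamera is a main menu actor that shows the menu and animates its own movement when play begins.
; On BeginPlay it creates the main menu widget, adds it to the viewport, switches input to UI only and shows the mouse cursor.
; A timeline then lerps the actor's location from a start position to an end position.
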(event `self.ReceiveBeginPlay`
  (bind _returnvalue (`GameplayStatics.GetPlayerController` 0))
  (bind _returnvalue_2 (`|CreateWidget` "/Game/Blueprints/Widgets/MainMenuWidget.MainMenuWidget_C" _returnvalue))
  (bind _output_get (set `self.Menu Widget` _returnvalue_2))
  (`UserWidget.AddToViewport` _output_get 0)
  (`WidgetBlueprintLibrary.SetInputMode_UIOnlyEx` _returnvalue _returnvalue_2)
  (set `PlayerController.bShowMouseCursor` true _returnvalue)
  (bind (_direction _openmovement) (`Timeline|CameraLerp`)
    (:`Update`
      (`self.K2_SetActorLocation` (`KismetMathLibrary.VLerp` (`self.StartPosition`) (`self.EndPosition`) _openmovement)))))

(fn `UserConstructionScript`)