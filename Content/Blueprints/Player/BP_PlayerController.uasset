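; Player controller that forwards movement and zoom input to the possessed BP_PlayerPawn.
; On BeginPlay it casts the controlled pawn and caches it.
; MoveRight and MoveUp axes pass scaled vectors on world X and Z to the pawn's Movement, giving planar side-view motion.
; The ZoomIn axis calls CameraZoom with a boolean for direction, ignoring zero input.
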(event `self.ReceiveBeginPlay`
  (`self.Init`))

(event `Init`
  (bind _asbp_player_pawn (cast `/Game/Blueprints/Player/BP_PlayerPawn` (`self.K2_GetPawn`)))
  (set `self.PlayerPawn` _asbp_player_pawn))

(event `InputAxis|MoveRight`
  (params (AxisValue :type "Float (single-precision)"))
  (`/Game/Blueprints/Player/BP_PlayerPawn.Movement` (`self.PlayerPawn`) (* (1000.0 0.0 0.0) AxisValue)))

(event `InputAxis|MoveUp`
  (params (AxisValue :type "Float (single-precision)"))
  (`/Game/Blueprints/Player/BP_PlayerPawn.Movement` (`self.PlayerPawn`) (* (0.0 0.0 1000.0) AxisValue)))

(event `InputAxis|ZoomIn`
  (params (AxisValue :type "Float (single-precision)"))
  (if (< AxisValue 0.0)
    (`/Game/Blueprints/Player/BP_PlayerPawn.CameraZoom` (`self.PlayerPawn`) false)
    (elif (> AxisValue 0.0)
      (`/Game/Blueprints/Player/BP_PlayerPawn.CameraZoom` (`self.PlayerPawn`) true))))

(fn `UserConstructionScript`)