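; Player pawn that acts as a movable camera, panning on the X/Z plane and zooming along Y.
; Movement feeds the vector to FloatingPawnMovement only when CheckCameraMovement finds a direction within bounds, passing the whole vector if any one qualifies.
; Bounds come from XBoundary, YBoundary (capping Z height) and a fixed Z floor.
; CameraZoom moves the pawn in fixed, swept Y steps within a symmetric range.
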(fn `CameraZoom`
  (params (Forward :type Boolean))
  (bind _floatingpawnmovement (`self.FloatingPawnMovement`))
  (bind (_returnvalue_x _returnvalue_y) (`KismetMathLibrary.BreakVector` (`SceneComponent.K2_GetComponentLocation` (`self.DefaultSceneRoot`))))
  (if Forward
    (if (< (+ _returnvalue_y 100.0) 600.0)
      (`MovementComponent.K2_MoveUpdatedComponent` :`self` _floatingpawnmovement :`Delta` (0.0 100.0 0.0)))
    (elif (> (- _returnvalue_y 100.0) -600.0)
      (`MovementComponent.K2_MoveUpdatedComponent` :`self` _floatingpawnmovement :`Delta` (0.0 -100.0 0.0)))))

(fn `Movement`
  (params (MovementVector :type "Vector Structure"))
  (`self.CheckCameraMovement` MovementVector
    (:`CanMove`
      (`PawnMovementComponent.AddInputVector` (`self.FloatingPawnMovement`) MovementVector false))))

(fn `UserConstructionScript`)