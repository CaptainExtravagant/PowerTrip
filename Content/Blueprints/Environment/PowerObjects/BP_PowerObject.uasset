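; BP_PowerObject is a clickable world object that toggles between powered and unpowered by trading power with a PowerManager.
; Clicking a powered object returns its PowerLevel to the manager; clicking an unpowered one takes that amount only if available, with a sound for each switch.
; The construction script applies the IsPowered state through EnablePower or DisablePower.
; ComparePowerLevel checks whether the manager's selected object has the same PowerLevel.
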(event `SetManager`
  (params (NewManager :type "/Game/Blueprints/Environment/PowerObjects/BP_PowerManager Object Reference"))
  (set `self.PowerManager` NewManager))

(event `self.ReceiveActorOnClicked`
  (params (ButtonPressed :type "Key Structure"))
  (`self.ObjectClicked`))

(event `self.ObjectClicked`
  (bind _powerlevel (`self.PowerLevel`))
  (bind _powermanager (`self.PowerManager`))
  (if (`self.IsPowered`)
    (`/Game/Blueprints/Environment/PowerObjects/BP_PowerManager.AddPower` _powermanager _powerlevel)
    (`self.DisablePower`)
    (`GameplayStatics.PlaySound2D` "/Game/Audio/SFX/PowerDown.PowerDown")
    (elif (`/Game/Blueprints/Environment/PowerObjects/BP_PowerManager.IsPowerAvailable` _powermanager _powerlevel)
      (`/Game/Blueprints/Environment/PowerObjects/BP_PowerManager.RemovePower` _powermanager _powerlevel)
      (`self.EnablePower`)
      (`GameplayStatics.PlaySound2D` "/Game/Audio/SFX/PowerOn.PowerOn"))))

(fn `ComparePowerLevel`
  (returns (EqualPower :type Boolean))
  (return (== (`/Game/Blueprints/Environment/PowerObjects/BP_PowerObject.PowerLevel` (`/Game/Blueprints/Environment/PowerObjects/BP_PowerManager.SelectedObject` (`self.PowerManager`))) (`self.PowerLevel`))))

(fn `UserConstructionScript`
  (if (`self.IsPowered`)
    (`self.EnablePower`)
    (else
      (`self.DisablePower`))))