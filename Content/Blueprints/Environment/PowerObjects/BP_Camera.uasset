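; BP_Camera is a powered security camera that signals its state by color through a cone mesh, a static mesh and a spotlight.
; EnablePower and DisablePower set IsPowered and switch the emissive materials and light color to green or blue.
; SpottedSpy turns them red without changing the power state; detection logic is not in these graphs.
; The construction script only calls the parent's.
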(event `SpottedSpy`
  (`PrimitiveComponent.SetMaterial` (`self.CameraCone`) 0 "/Game/Art/Materials/Environment/M_Red_Emissive.M_Red_Emissive")
  (`PrimitiveComponent.SetMaterial` (`self.StaticMesh`) 0 "/Game/Art/Materials/Environment/M_Red_Emissive.M_Red_Emissive")
  (`LightComponent.SetLightColor` (`self.SpotLight`) (struct :`R` 1.0 :`A` 1.0) true))

(event `/Game/Blueprints/Environment/PowerObjects/I_PowerObject.EnablePower`
  (set `self.IsPowered` true)
  (`PrimitiveComponent.SetMaterial` (`self.CameraCone`) 0 "/Game/Art/Materials/Environment/M_Green_Emissive.M_Green_Emissive")
  (`PrimitiveComponent.SetMaterial` (`self.StaticMesh`) 0 "/Game/Art/Materials/Environment/M_Green_Emissive.M_Green_Emissive")
  (`LightComponent.SetLightColor` (`self.SpotLight`) (struct :`G` 1.0 :`A` 1.0) true))

(event `/Game/Blueprints/Environment/PowerObjects/I_PowerObject.DisablePower`
  (set `self.IsPowered` false)
  (`PrimitiveComponent.SetMaterial` (`self.CameraCone`) 0 "/Game/Art/Materials/Environment/M_Blue_Emissive.M_Blue_Emissive")
  (`PrimitiveComponent.SetMaterial` (`self.StaticMesh`) 0 "/Game/Art/Materials/Environment/M_Blue_Emissive.M_Blue_Emissive")
  (`LightComponent.SetLightColor` (`self.SpotLight`) (struct :`B` 1.0 :`A` 1.0) true))

(fn `UserConstructionScript`
  (`parent.UserConstructionScript`))