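; BP_Light is a powered spotlight that can act as a distraction for guards.
; PartnerObjectFound toggles power by showing or hiding the SpotLight and updating IsPowered.
; When disabled with CanBeDistraction set, it calls ChangeRootMessage on GuardRef with RootToChangeToo.
; GuardRef is cached shortly after BeginPlay by looping over all BaseGuardClass actors, so only the last guard found receives that message.
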(event `self.ReceiveBeginPlay`
  (`KismetSystemLibrary.Delay` 0.2)
  (bind _outactors (`GameplayStatics.GetAllActorsOfClass` "/Game/Blueprints/Guards/BaseGuardClass.BaseGuardClass_C"))
  (for _array_element _outactors
    (set `self.GuardRef` _array_element)))

(event `self.PartnerObjectFound`
  (params (PartnerObject :type "/Game/Blueprints/Environment/PowerObjects/BP_PowerObject Object Reference"))
  (if (`self.IsPowered`)
    (`self.DisablePower`)
    (else
      (`self.EnablePower`))))

(event `self.EnablePower`
  (`SceneComponent.SetVisibility` (`self.SpotLight`) true false)
  (set `self.IsPowered` true))

(event `self.DisablePower`
  (`SceneComponent.SetVisibility` (`self.SpotLight`) false false)
  (set `self.IsPowered` false)
  (if (`self.CanBeDistraction`)
    (message `/Game/Blueprints/Interfaces/iNpcSystem.ChangeRoot` (`self.GuardRef`) (`self.RootToChangeToo`))))

(fn `UserConstructionScript`
  (`parent.UserConstructionScript`))