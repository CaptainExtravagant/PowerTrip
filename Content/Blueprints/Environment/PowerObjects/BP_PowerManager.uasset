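; BP_PowerManager tracks a shared pool of available power for the power objects in the level.
; On BeginPlay it gathers every BP_PowerObject into an array and registers itself as their manager.
; It exposes functions to check, add and remove power, and to store the currently selected object.
; The remove function does a plain subtraction; the availability check is a separate call.
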(event `Init`
  (bind _outactors (`GameplayStatics.GetAllActorsOfClass` "/Game/Blueprints/Environment/PowerObjects/BP_PowerObject.BP_PowerObject_C"))
  (bind _output_get (set `self.A_PowerObjects` _outactors))
  (for _array_element _output_get
    (`/Game/Blueprints/Environment/PowerObjects/BP_PowerObject.SetManager` _array_element self)))

(event `self.ReceiveBeginPlay`
  (`self.Init`))

(fn `AddPower`
  (params (PowerToAdd :type Integer))
  (set `self.AvailablePower` (+ (`self.AvailablePower`) PowerToAdd)))

(fn `IsPowerAvailable`
  (params (PowerNeeded :type Integer))
  (returns (PowerAvailable :type Boolean))
  (return (<= PowerNeeded (`self.AvailablePower`))))

(fn `RemovePower`
  (params (PowerToRemove :type Integer))
  (set `self.AvailablePower` (- (`self.AvailablePower`) PowerToRemove)))

(fn `SetSelectedObject`
  (params (NewObject :type "/Game/Blueprints/Environment/PowerObjects/BP_PowerObject Object Reference"))
  (set `self.SelectedObject` NewObject))

(fn `UserConstructionScript`)