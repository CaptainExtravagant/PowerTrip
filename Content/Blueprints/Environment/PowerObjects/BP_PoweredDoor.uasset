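; Powered door that swings between open and closed poses and shows its state with a green or red point light.
; EnablePower and DisablePower open or close it according to the PoweredOpen setting.
; Front and back colliders share logic: guards open a closed, powered door, which shuts on a short timer.
; A spy overlapping either collider while the door is closed triggers AgentDiscovered on the GM_Base game mode.
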(event `/Game/Blueprints/Environment/PowerObjects/I_PowerObject.DisablePower`
  (set `self.IsPowered` false)
  (if (`self.PoweredOpen`)
    (`self.CloseDoor`)
    (else
      (`self.OpenDoor`))))

(event `/Game/Blueprints/Environment/PowerObjects/I_PowerObject.EnablePower`
  (set `self.IsPowered` true)
  (if (`self.PoweredOpen`)
    (`self.OpenDoor`)
    (else
      (`self.CloseDoor`))))

(event `self.FrontCollider.OnComponentBeginOverlap`
  (params (OverlappedComponent :type "PrimitiveComponent Object Reference") (OtherActor :type "Actor Object Reference") (OtherComp :type "PrimitiveComponent Object Reference") (OtherBodyIndex :type Integer) (bFromSweep :type Boolean) (SweepResult :type "HitResult Structure (by ref)"))
  (if (`.bSuccess` (cast `/Game/Blueprints/Guards/BaseGuardClass` OtherActor :!pure true))
    (if (`self.IsOpen`) :!label _label
      _
      (elif (`self.IsPowered`)
        (`self.OpenDoor`)
        (`KismetSystemLibrary.K2_SetTimer` null "CloseDoor" 2.0)))
    (else
      (cast `/Game/Blueprints/Spy/BaseSpyClass` OtherActor)
      (if (not (`self.IsOpen`)) :!label _label_2
        (`/Game/Blueprints/GM_Base.AgentDiscovered` (cast `/Game/Blueprints/GM_Base` (`GameplayStatics.GetGameMode`) :!pure true))))))

(event `self.BackCollider.OnComponentBeginOverlap`
  (params (OverlappedComponent :type "PrimitiveComponent Object Reference") (OtherActor :type "Actor Object Reference") (OtherComp :type "PrimitiveComponent Object Reference") (OtherBodyIndex :type Integer) (bFromSweep :type Boolean) (SweepResult :type "HitResult Structure (by ref)"))
  (if (`.bSuccess` (cast `/Game/Blueprints/Guards/BaseGuardClass` OtherActor :!pure true))
    (goto _label)
    (else
      (cast `/Game/Blueprints/Spy/BaseSpyClass` OtherActor)
      (goto _label_2))))

(fn `CloseDoor`
  (bind _staticmesh (`self.StaticMesh`))
  (bind (_returnvalue_location _returnvalue_rotation _returnvalue_scale) (`KismetMathLibrary.BreakTransform` (`SceneComponent.GetRelativeTransform` _staticmesh)))
  (`LightComponent.SetLightColor` (`self.PointLight`) (struct :`R` 1.0 :`A` 1.0) true)
  (set `self.IsOpen` false)
  (`SceneComponent.K2_SetRelativeTransform` _staticmesh (`KismetMathLibrary.MakeTransform` (0.0 -40.0 0.0) (struct) _returnvalue_scale) false false))

(fn `OpenDoor`
  (bind _staticmesh (`self.StaticMesh`))
  (`LightComponent.SetLightColor` (`self.PointLight`) (struct :`G` 1.0 :`A` 1.0) true)
  (set `self.IsOpen` true)
  (`SceneComponent.K2_SetRelativeTransform` _staticmesh (`KismetMathLibrary.MakeTransform` (-160.0 -100.0 0.0) (struct :`Yaw` -90.0) (`SceneComponent.RelativeScale3D` _staticmesh)) false false))

(fn `UserConstructionScript`
  (`parent.UserConstructionScript`))