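; BP_Door is a door that opens when anything begins overlapping its front or back collider and closes on a two-second timer.
; OpenDoor and CloseDoor set the Open flag and snap the mesh between two relative transforms, with no animation.
; The construction script applies the pose matching Open, so the initial state can be set per instance.
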(event `self.Front Collider.OnComponentBeginOverlap`
  (params (OverlappedComponent :type "PrimitiveComponent Object Reference") (OtherActor :type "Actor Object Reference") (OtherComp :type "PrimitiveComponent Object Reference") (OtherBodyIndex :type Integer) (bFromSweep :type Boolean) (SweepResult :type "HitResult Structure (by ref)"))
  (`self.OpenDoor` :!label _label)
  (`KismetSystemLibrary.K2_SetTimer` null "CloseDoor" 2.0))

(event `self.BackCollider.OnComponentBeginOverlap`
  (params (OverlappedComponent :type "PrimitiveComponent Object Reference") (OtherActor :type "Actor Object Reference") (OtherComp :type "PrimitiveComponent Object Reference") (OtherBodyIndex :type Integer) (bFromSweep :type Boolean) (SweepResult :type "HitResult Structure (by ref)"))
  (goto _label))

(fn `CloseDoor`
  (bind _staticmesh (`self.StaticMesh`))
  (bind (_returnvalue_location _returnvalue_rotation _returnvalue_scale) (`KismetMathLibrary.BreakTransform` (`SceneComponent.GetRelativeTransform` _staticmesh)))
  (set `self.Open` false)
  (`SceneComponent.K2_SetRelativeTransform` _staticmesh (`KismetMathLibrary.MakeTransform` (0.0 -40.0 0.0) (struct) _returnvalue_scale) false false))

(fn `OpenDoor`
  (bind _staticmesh (`self.StaticMesh`))
  (set `self.Open` true)
  (`SceneComponent.K2_SetRelativeTransform` _staticmesh (`KismetMathLibrary.MakeTransform` (-40.0 0.0 0.0) (struct :`Yaw` -90.0) (`SceneComponent.RelativeScale3D` _staticmesh)) false false))

(fn `UserConstructionScript`
  (if (`self.Open`)
    (`self.OpenDoor`)
    (else
      (`self.CloseDoor`))))