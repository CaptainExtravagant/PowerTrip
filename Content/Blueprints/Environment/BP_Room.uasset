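; BP_Room is a room volume that reports an agent as discovered when a spy enters while one of its cameras is powered.
; RoomOverlap events maintain the list of overlapping BaseSpyClass characters, and each spy entry runs CheckForIntruders.
; That check loops over OwnedObjects and calls AgentDiscovered on GM_Base for powered BP_Camera objects, without testing line of sight.
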(event `self.RoomOverlap.OnComponentBeginOverlap`
  (params (OverlappedComponent :type "PrimitiveComponent Object Reference") (OtherActor :type "Actor Object Reference") (OtherComp :type "PrimitiveComponent Object Reference") (OtherBodyIndex :type Integer) (bFromSweep :type Boolean) (SweepResult :type "HitResult Structure (by ref)"))
  (bind _asbase_spy_class (cast `/Game/Blueprints/Spy/BaseSpyClass` OtherActor))
  (`KismetArrayLibrary.Array_AddUnique` (`self.OverlappingCharacters`) _asbase_spy_class)
  (`self.CheckForIntruders`))

(event `self.RoomOverlap.OnComponentEndOverlap`
  (params (OverlappedComponent :type "PrimitiveComponent Object Reference") (OtherActor :type "Actor Object Reference") (OtherComp :type "PrimitiveComponent Object Reference") (OtherBodyIndex :type Integer))
  (bind _asbase_spy_class (cast `/Game/Blueprints/Spy/BaseSpyClass` OtherActor))
  (`KismetArrayLibrary.Array_RemoveItem` (`self.OverlappingCharacters`) _asbase_spy_class))

(fn `CheckForIntruders`
  (for _array_element (`self.OwnedObjects`)
    (bind _asbp_camera (cast `/Game/Blueprints/Environment/BP_Camera` _array_element))
    (if (`/Game/Blueprints/Environment/BP_PowerObject.IsPowered` _asbp_camera)
      (bind _asgm_base (cast `/Game/Blueprints/GM_Base` (`GameplayStatics.GetGameMode`)))
      (`/Game/Blueprints/GM_Base.AgentDiscovered` _asgm_base))))

(fn `UserConstructionScript`)