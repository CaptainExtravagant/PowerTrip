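; BP_PoweredDoor is a door whose open state follows its power, with PoweredOpen choosing whether power opens or closes it.
; EnablePower and DisablePower update IsPowered and call OpenDoor or CloseDoor, which only set IsOpen and swap between green and red materials.
; Front and back colliders detect BaseGuardClass actors, opening a closed, powered door and closing it on a short timer.
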(event `/Game/Blueprints/Environment/I_PowerObject.DisablePower`
  (set `self.IsPowered` false)
  (if (`self.PoweredOpen`)
    (`self.CloseDoor`)
    (else
      (`self.OpenDoor`))))

(event `/Game/Blueprints/Environment/I_PowerObject.EnablePower`
  (set `self.IsPowered` true)
  (if (`self.PoweredOpen`)
    (`self.OpenDoor`)
    (else
      (`self.CloseDoor`))))

(event `self.FrontCollider.OnComponentBeginOverlap`
  (params (OverlappedComponent :type "PrimitiveComponent Object Reference") (OtherActor :type "Actor Object Reference") (OtherComp :type "PrimitiveComponent Object Reference") (OtherBodyIndex :type Integer) (bFromSweep :type Boolean) (SweepResult :type "HitResult Structure (by ref)"))
  (if (`.bSuccess` (cast `/Game/Blueprints/Guards/BaseGuardClass` OtherActor :!pure true))
    (if (`self.IsOpen`) :!label _label
      _
      (elif (`self.IsPowered`)
        (`self.OpenDoor`)
        (`KismetSystemLibrary.K2_SetTimer` null "CloseDoor" 2.0)))))

(event `self.BackCollider.OnComponentBeginOverlap`
  (params (OverlappedComponent :type "PrimitiveComponent Object Reference") (OtherActor :type "Actor Object Reference") (OtherComp :type "PrimitiveComponent Object Reference") (OtherBodyIndex :type Integer) (bFromSweep :type Boolean) (SweepResult :type "HitResult Structure (by ref)"))
  (if (`.bSuccess` (cast `/Game/Blueprints/Guards/BaseGuardClass` OtherActor :!pure true))
    (goto _label)))

(fn `CloseDoor`
  (`PrimitiveComponent.SetMaterial` (`self.StaticMesh`) 0 "/Game/Art/Materials/M_Red.M_Red")
  (set `self.IsOpen` false))

(fn `OpenDoor`
  (`PrimitiveComponent.SetMaterial` (`self.StaticMesh`) 0 "/Game/Art/Materials/M_Green.M_Green")
  (set `self.IsOpen` true))

(fn `UserConstructionScript`
  (`parent.UserConstructionScript`))