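; Base environment object for a power system, holding a powered state and a power level and working with a power manager.
; The construction script calls EnablePower or DisablePower to match IsPowered.
; A click on the actor triggers ObjectClicked, and SetManager stores the manager reference.
; ComparePowerLevel checks whether the manager's selected object has the same power level as this one.
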(event `SetManager`
  (params (NewManager :type "/Game/Blueprints/Environment/BP_PowerManager Object Reference"))
  (set `self.PowerManager` NewManager))

(event `self.ReceiveActorOnClicked`
  (params (ButtonPressed :type "Key Structure"))
  (`self.ObjectClicked`))

(fn `ComparePowerLevel`
  (returns (EqualPower :type Boolean))
  (return (== (`/Game/Blueprints/Environment/BP_PowerObject.PowerLevel` (`/Game/Blueprints/Environment/BP_PowerManager.SelectedObject` (`self.PowerManager`))) (`self.PowerLevel`))))

(fn `UserConstructionScript`
  (if (`self.IsPowered`)
    (`self.EnablePower`)
    (else
      (`self.DisablePower`))))