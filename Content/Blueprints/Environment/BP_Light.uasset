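; BP_Light is an environment light that switches its SpotLight on and off as a powered object.
; Its PartnerObjectFound event acts as a toggle, calling EnablePower or DisablePower based on the IsPowered flag.
; Those two events set the spotlight's visibility and update IsPowered to match.
; The construction script only runs the parent's version.
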(event `self.PartnerObjectFound`
  (params (PartnerObject :type "/Game/Blueprints/Environment/BP_PowerObject Object Reference"))
  (if (`self.IsPowered`)
    (`self.DisablePower`)
    (else
      (`self.EnablePower`))))

(event `self.EnablePower`
  (`SceneComponent.SetVisibility` (`self.SpotLight`) true false)
  (set `self.IsPowered` true))

(event `self.DisablePower`
  (`SceneComponent.SetVisibility` (`self.SpotLight`) false false)
  (set `self.IsPowered` false))

(fn `UserConstructionScript`
  (`parent.UserConstructionScript`))