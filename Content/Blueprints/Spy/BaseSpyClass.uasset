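; Base spy actor that moves along a supplied spline and halts at designated spline points.
; A looping timer advances its distance along the spline each tick and stops at the spline's end.
; Reaching a listed stop point clears the timer, with a short cooldown before stops are checked again.
; On BeginPlay it binds an event to the end-turn dispatcher through the player pawn's controller.
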(event `self.ReceiveBeginPlay`
  ;[1 1 1] Bind self to controller
  (bind _controller_ref (message `/Game/Blueprints/Interfaces/iControllerRefSystem.ControllerRefSelf` (`Pawn.GetController` (`GameplayStatics.GetPlayerPawn` 0))))
  (add `/Game/Blueprints/Player/BP_PlayerController.EndTurnDispatcher` _controller_ref (`|CreateDelegate` :!event `StartMoveTimer`)))

(event `StartMoveTimer`
  ;[1 1 1] Start moving the spy
  (bind _returnvalue (`KismetSystemLibrary.K2_SetTimerDelegate` (delegate `MoveSpy`) 0.1 true :!label _label))
  (set `self.MoveTimer` _returnvalue))

(event `/Game/Blueprints/Interfaces/iSpySystem.SpyGetSpline`
  (params (Spline :type "SplineComponent Object Reference") (SplinesToStopAt :type "Array of Integer (by ref)"))
  ;[1 1 1] Start moving the spy
  (set `self.Spine` Spline)
  (set `self.SplinePointsToStopAt` SplinesToStopAt)
  (goto _label))

(event `MoveSpy`
  ;[1 1 1] Move Along spline
  (bind _output_get (set `self.DistanceAlongSpline` (+ (`self.DistanceAlongSpline`) (`self.MovementSpeed`))))
  (`self.K2_SetActorTransform` (`KismetMathLibrary.MakeTransform` (`SplineComponent.GetLocationAtDistanceAlongSpline` (`self.Spine`) _output_get "World") (struct) (1.0 1.0 1.0)))
  (`self.CheckLocation`)
  (if (>= (`self.DistanceAlongSpline`) (`SplineComponent.GetSplineLength` (`self.Spine`)))
    (`KismetSystemLibrary.K2_ClearAndInvalidateTimerHandle` (`self.MoveTimer`))))

(event `CheckLocation`
  ;[1 1 1] Check to see if spy is within a spline point and if so stop them
  (if (and (`self.CanStop`) (`KismetMathLibrary.NearlyEqual_TransformTransform` (`SceneComponent.K2_GetComponentToWorld` (`self.DefaultSceneRoot`)) (`SplineComponent.GetTransformAtSplinePoint` (`self.Spine`) (`self.NextSplinePoint`) "World" false) 50.0 50.0 50.0))
    (for _array_element (`self.SplinePointsToStopAt`)
      (if (== _array_element (`self.NextSplinePoint`))
        (set `self.SplinePointMatch` true)
        (break)))
    (if (`self.SplinePointMatch`)
      (`KismetSystemLibrary.K2_ClearAndInvalidateTimerHandle` (`self.MoveTimer`))
      (`/Engine/EditorBlueprintResources/StandardMacros.IncrementInt` (`self.NextSplinePoint`)
        (:`  `
          (set `self.CanStop` false)
          (set `self.SplinePointMatch` false)
          (`KismetSystemLibrary.Delay` 1.0)
          (set `self.CanStop` true)))
      (else
        (`/Engine/EditorBlueprintResources/StandardMacros.IncrementInt` (`self.NextSplinePoint`))))))

(fn `UserConstructionScript`)