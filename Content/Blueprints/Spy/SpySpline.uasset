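; SpySpline is a spline actor that spawns a Spy when play begins and hands it a path to follow.
; On BeginPlay it spawns the Spy at the start of its spline, owned by this actor and with zero rotation.
; It then sends the spawned Spy the spline and its SplinesToStopAt data through the SpyGetSplineMessage call.
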(event `self.ReceiveBeginPlay`
  (`self.Spawn Spy`))

(event `Spawn Spy`
  ;[1 1 1] Spawn spy and give them the spline
  (set `self.DistanceAlongSpline` 0.0)
  (bind _returnvalue (`|SpawnActorFromClass` (`self.Spy`) (`KismetMathLibrary.MakeTransform` (`SplineComponent.GetLocationAtDistanceAlongSpline` (`self.Spline`) (`self.DistanceAlongSpline`) "World")) "Undefined" "OverrideRootScale" self null))
  (message `/Game/Blueprints/Interfaces/iSpySystem.SpyGetSpline` _returnvalue (`self.Spline`) (`self.SplinesToStopAt`)))

(fn `UserConstructionScript`)