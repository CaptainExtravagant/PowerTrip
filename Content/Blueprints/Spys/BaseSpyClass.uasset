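; BaseSpyClass is a base spy actor that travels along a spline handed to it through SpyGetSpline.
; That event stores the spline and starts a looping timer, keeping its handle, to step movement at a fixed interval instead of on Tick.
; Each step adds MoveAmount to the travelled distance and sets the actor to that world-space spline point without sweeping, with rotation zeroed and unit scale.
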(event `/Game/Blueprints/Interfaces/iSpySystem.SpyGetSpline`
  (params (Spline :type "SplineComponent Object Reference"))
  (set `self.Spline` Spline)
  (bind _returnvalue (`KismetSystemLibrary.K2_SetTimerDelegate` (delegate `MoveAlongSpline`) 0.1 true))
  (set `self.MovementTimer` _returnvalue))

(event `MoveAlongSpline`
  (bind _output_get (set `self.DistanceAlongSpline` (+ (`self.MoveAmount`) (`self.DistanceAlongSpline`))))
  (`self.K2_SetActorTransform` (`KismetMathLibrary.MakeTransform` (`SplineComponent.GetLocationAtDistanceAlongSpline` (`self.Spline`) _output_get "World"))))

(fn `UserConstructionScript`)