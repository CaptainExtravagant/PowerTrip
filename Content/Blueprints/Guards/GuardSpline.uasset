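; GuardSpline is a spline path actor that spawns a guard to use that path.
; On BeginPlay, if CanSpawnGuard is set, it spawns the guard at the spline's start in world space, with itself as owner.
; It then passes the spline and SplinesToStopAt to the guard through NpcGetSplineMessage, leaving any movement along the path to the guard.
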(event `self.ReceiveBeginPlay`
  ;[1 1 1] If can spawn guard then start spawing the guard
  (if (`self.CanSpawnGuard`)
    (`self.SpawnGuard`)))

(event `SpawnGuard`
  ;[1 1 1] Spawn guard and pass them the spline
  (set `self.DistanceAlongSpline` 0.0)
  (bind _returnvalue (`|SpawnActorFromClass` (`self.Guard`) (`KismetMathLibrary.MakeTransform` (`SplineComponent.GetLocationAtDistanceAlongSpline` (`self.Spline`) (`self.DistanceAlongSpline`) "World")) "Undefined" "OverrideRootScale" self null))
  (message `/Game/Blueprints/Interfaces/iNpcSystem.NpcGetSpline` _returnvalue (`self.Spline`) (`self.SplinesToStopAt`)))

(fn `UserConstructionScript`)