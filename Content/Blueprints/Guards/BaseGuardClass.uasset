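; Base guard Blueprint that patrols back and forth along a spline between the ends of its patrol route.
; A looping timer advances the guard by distance, then compares its transform with the next spline point to update point indices.
; At designated stop points it clears the timer until movement is restarted.
; It binds to the player controller's end-turn dispatcher and exposes a direction-swap event.
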(event `/Game/Blueprints/Interfaces/iNpcSystem.NpcGetPotrolRoot`
  (params (Root1 :type "Array of Integer (by ref)"))
  (set `self.PotrolRoot1` Root1)
  (bind _output_get (set `self.CurrentPotrolRoot` Root1))
  (bind _output (`|GetArrayItem` _output_get))
  (set `self.CurrentSplinePoint` (- _output 1))
  (set `self.NextSplinePoint` _output))

(event `self.ReceiveBeginPlay`
  ;[1 1 1] Bind self to controller
  (bind _controller_ref (message `/Game/Blueprints/Interfaces/iControllerRefSystem.ControllerRefSelf` (`Pawn.GetController` (`GameplayStatics.GetPlayerPawn` 0))))
  (add `/Game/Blueprints/Player/BP_PlayerController.EndTurnDispatcher` _controller_ref (`|CreateDelegate` :!event `StartMoveTimer`)))

(event `StartMoveTimer`
  ;[1 1 1] Start moving the Guard
  (bind _returnvalue (`KismetSystemLibrary.K2_SetTimerDelegate` (delegate `MoveSpy`) 0.1 true :!label _label))
  (set `self.MoveTimer` _returnvalue))

(event `/Game/Blueprints/Interfaces/iNpcSystem.NpcGetSpline`
  (params (Spline :type "SplineComponent Object Reference") (SplineToStopAt :type "Array of Integer (by ref)") (StartDistance :type "Float (single-precision)"))
  ;[1 1 1] Start moving the Guard
  (set `self.Spine` Spline)
  (set `self.SplinePointsToStopAt` SplineToStopAt)
  (set `self.DistanceAlongSpline` StartDistance)
  (goto _label))

(event `MoveSpy`
  (bind _distancealongspline (`self.DistanceAlongSpline`))
  (bind _movementspeed (`self.MovementSpeed`))
  (bind _currentpotrolroot (`self.CurrentPotrolRoot`))
  (bind _currentpotrolroot_2 (`self.CurrentPotrolRoot`))
  (bind _currentpotrolroot_3 (`self.CurrentPotrolRoot`))
  ;[1 1 1] Move Along spline
  (if (`self.IsMoveForward`)
    (bind _output_get (set `self.DistanceAlongSpline` (+ _distancealongspline _movementspeed)))
    (`self.MoveAlongSpline` _output_get)
    (if (== (`|GetArrayItem` _currentpotrolroot_2 (`KismetArrayLibrary.Array_LastIndex` _currentpotrolroot_2)) (`self.CurrentSplinePoint`))
      (set `self.IsMoveForward` false)
      (set `self.NextSplinePoint` (- (`|GetArrayItem` _currentpotrolroot_3 (`KismetArrayLibrary.Array_LastIndex` _currentpotrolroot_3)) 1))
      (set `self.CurrentSplinePoint` (`|GetArrayItem` _currentpotrolroot (`KismetArrayLibrary.Array_LastIndex` _currentpotrolroot))))
    (else
      (bind _output_get_2 (set `self.DistanceAlongSpline` (- _distancealongspline _movementspeed)))
      (`self.MoveAlongSpline` _output_get_2)
      (if (== (`|GetArrayItem` _currentpotrolroot_2) (`self.CurrentSplinePoint`))
        (set `self.IsMoveForward` true)
        (set `self.NextSplinePoint` (+ (`|GetArrayItem` (`self.CurrentPotrolRoot`)) 1))
        (set `self.CurrentSplinePoint` (`|GetArrayItem` (`self.CurrentPotrolRoot`)))))))

(event `SwapDirection`
  (bind _nextsplinepoint (`self.NextSplinePoint`))
  ;[1 1 1] Swap direction
  (if (`self.IsMoveForward`)
    (set `self.IsMoveForward` false)
    (set `self.NextSplinePoint` (- _nextsplinepoint 2))
    (else
      (set `self.IsMoveForward` true)
      (set `self.NextSplinePoint` (+ _nextsplinepoint 2)))))

(event `CheckLocation`
  ;[1 1 1] Check to see if Guard is within a spline point and if so stop them
  (if (and (`self.CanStop`) (`KismetMathLibrary.NearlyEqual_TransformTransform` (`SceneComponent.K2_GetComponentToWorld` (`self.DefaultSceneRoot`)) (`SplineComponent.GetTransformAtSplinePoint` (`self.Spine`) (`self.NextSplinePoint`) "World" false) 50.0 50.0 50.0))
    (`/Engine/EditorBlueprintResources/StandardMacros.DoOnce` false :!label _label_2
      (:`Completed`
        (if (`KismetArrayLibrary.Array_Contains` (`self.SplinePointsToStopAt`) (`self.NextSplinePoint`))
          (`KismetSystemLibrary.K2_ClearAndInvalidateTimerHandle` (`self.MoveTimer`))
          (`self.ManagePoints`)
          (set `self.CanStop` false)
          (set `self.SplinePointMatch` false)
          (`KismetSystemLibrary.Delay` 2.0)
          (set `self.CanStop` true)
          (goto _label_2 :!via `Reset`)
          (else
            (`self.ManagePoints`)
            (`KismetSystemLibrary.Delay` 2.0)
            (goto _label_2 :!via `Reset`)))))))

(fn `ManagePoints`
  (returns (Ignore :type Boolean))
  (bind _nextsplinepoint (`self.NextSplinePoint`))
  (bind _currentsplinepoint (`self.CurrentSplinePoint`))
  (if (`self.IsMoveForward`)
    (`/Engine/EditorBlueprintResources/StandardMacros.IncrementInt` _nextsplinepoint
      (:`  `
        (`/Engine/EditorBlueprintResources/StandardMacros.IncrementInt` _currentsplinepoint
          (:`  `
            _))))
    (else
      (`/Engine/EditorBlueprintResources/StandardMacros.DecrementInt` _nextsplinepoint
        (:`  `
          (`/Engine/EditorBlueprintResources/StandardMacros.DecrementInt` _currentsplinepoint
            (:`  `
              _))))))
  (return false))

(fn `MoveAlongSpline`
  (params (Distance :type "Float (double-precision)"))
  (returns (ignore :type Boolean))
  (`self.K2_SetActorTransform` (`KismetMathLibrary.MakeTransform` (`SplineComponent.GetLocationAtDistanceAlongSpline` (`self.Spine`) Distance "World")))
  (`self.CheckLocation`)
  (return false))

(fn `UserConstructionScript`)